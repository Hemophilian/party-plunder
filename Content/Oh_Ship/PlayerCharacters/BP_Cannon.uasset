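; Player-controlled cannon that shoots targets to earn gold, with aiming, rotation reset and a pause menu.
; Axis input rotates the base pivot; a DoOnce-gated fire plays a montage, then spawns a cannonball after a delay.
; A separate muzzle line trace, not the projectile, triggers target hits, scoring by colour (Sea Serpant zeroes it) and updating the gold widget.
; A toggleable aim-assist beam is repositioned and stretched along the muzzle direction on Tick.
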(event Custom|FireCannon
  (bind _muzzlepoint (Variables|Default|GetMuzzlePoint))
  (bind _arrow (Variables|Default|GetArrow))
  (bind _returnvalue (Transformation|GetWorldLocation _muzzlepoint))
  (bind _returnvalue_2 (Transformation|GetWorldTransform _arrow))
  ;[1 0.8856 0] Cannon Fire and point setting
  (Game|SpawnActorfromClass "/Game/Oh_Ship/PlayerCharacters/BP_Cannonball_Cannon.BP_Cannonball_Cannon_C" (Math|Transform|MakeTransform (.location _returnvalue_2) (.rotation _returnvalue_2) "1.000000,1.000000,1.000000") "AlwaysSpawn" "MultiplyWithRoot" 0 0)
  (Utilities|FlowControl|Delay 0.2)
  (bind _outhit (Collision|LineTraceByChannel _returnvalue (+ _returnvalue (* (Math|Vector|GetForwardVector _muzzlepoint) (Variables|Default|GetShootDistance))) "TraceTypeQuery1" false 0 "ForDuration"))
  (Development|PrintString (Utilities|GetDisplayName (.HitActor (Collision|BreakHitResult _outhit))))
  (bind _asbp_targets (Utilities|Casting|CastToBP_Targets (.HitActor (Collision|BreakHitResult _outhit))))
  (Default|TakingFire! _asbp_targets)
  (if (>= (Variables|Default|GetHits) 0)
    (switch string (Utilities|String|EnumtoString (Variables|/Game/Oh_Ship/Targets/BP_Targets.BP_Targets_C|GetTarget%20Colour _asbp_targets))
      (:Default
        (Variables|Default|SetTargetValue 20 :!label _label)
        (bind _output_get (Variables|Default|SetHits (+ (Variables|Default|GetHits) (Variables|Default|GetTargetValue)) :!label _label_2)))
      (:Red
        (goto _label))
      (:Bue
        (Variables|Default|SetTargetValue 40)
        (goto _label_2))
      (:Green
        (Variables|Default|SetTargetValue 30)
        (goto _label_2))
      (:Sea%20Serpant
        (Variables|Default|SetHits (- (Variables|Default|GetHits) (Variables|Default|GetHits)))))
    (bind _aswbp_player_gold_display (Utilities|Casting|CastToWBP_PlayerGoldDisplay (UserInterface|GetUserWidgetObject (Variables|Default|GetSuccessfullHits))))
    (Variables|/Script/UMG.TextBlock|SetText (Variables|/Game/TopDown/Blueprints/FatKingChase_Blueprints/WBP_PlayerGoldDisplay.WBP_PlayerGoldDisplay_C|GetGoldCount _aswbp_player_gold_display) (Utilities|Text|ToText(Integer) _output_get))))

(event Custom|Refire
  ;[0.05404 0.15 0.08285 0.5] Fire cannon with delay to time the animation
  (Utilities|FlowControl|DoOnce false) ; enters at Reset
)

(event Input|EnhancedActionEvents|EnhancedInputActionIA_Pause
  (params (ActionValue :type Boolean) (ElapsedSeconds :type Float%20%28double-precision%29) (TriggeredSeconds :type Float%20%28double-precision%29) (InputAction :type Input%20Action%20Object%20Reference :default "/Game/TopDown/Input/Actions/IA_Pause.IA_Pause"))
  (bind _returnvalue (Game|GetPlayerController 0))
  ;[0.15 0.07312 0.1388 0.5] Pause Menu
  (:Started
    (if (not (Variables|Default|GetIsPaused))
      (Variables|Default|SetIsPaused true)
      (bind _returnvalue_2 (UserInterface|CreateWidget "/Game/TopDown/Blueprints/FatKingChase_Blueprints/WBP_PauseMenu.WBP_PauseMenu_C" _returnvalue))
      (bind _output_get (Variables|Default|SetPause%20Menu%20Widget _returnvalue_2))
      (UserInterface|Viewport|AddtoViewport _output_get 0)
      (Input|SetInputModeGameandUI _returnvalue 0 "DoNotLock" true false)
      (Utilities|FlowControl|Delay 0.2)
      (Widget|SetKeyboardFocus (Variables|/Game/TopDown/Blueprints/FatKingChase_Blueprints/WBP_PauseMenu.WBP_PauseMenu_C|GetResumeButton _output_get))
      (Game|SetGamePaused true)
      (else
        (Variables|Default|SetIsPaused false)
        (Widget|RemovefromParent (Variables|Default|GetPause%20Menu%20Widget))
        (Game|SetGamePaused false)))))

(event EventBeginPlay
  ;[1 0.0735 0] Getting the begining rotation for reset
  (Variables|Default|SetInitialRotation (Transformation|GetWorldRotation (Variables|Default|GetCannonBody))))

(event EventTick
  (params (DeltaSeconds :type Float%20%28single-precision%29))
  ;[0 0 0] Aiming Assist Beam (Got me stumped but it does the job)
  (if (Variables|Default|GetAssistOn)
    (Variables|Default|SetStart (Transformation|GetWorldLocation (Variables|Default|GetMuzzlePoint)))
    (Variables|Default|SetForward (Math|Vector|GetForwardVector (Variables|Default|GetMuzzlePoint)))
    (Variables|Default|SetEnd (+ (Variables|Default|GetStart) (* (Variables|Default|GetForward) (Variables|Default|GetBeamLength))))
    (Variables|Default|SetMid (/ (+ (Variables|Default|GetStart) (Variables|Default|GetEnd)) (Variables|Default|GetNum)))
    (Variables|Default|SetDistance (Math|Vector|VectorLength (- (Variables|Default|GetEnd) (Variables|Default|GetStart))))
    (Transformation|SetWorldLocation (Variables|Default|GetAimBeam) (Variables|Default|GetMid) false false)
    (Transformation|SetWorldRotation (Variables|Default|GetAimBeam) (Math|Rotator|FindLookatRotation (Variables|Default|GetMid) (Variables|Default|GetEnd)) false false)
    (Transformation|SetWorldScale3D (Variables|Default|GetAimBeam) (Math|Vector|MakeVector (/ (Variables|Default|GetDistance) 1e+01) 0.02 0.02))))

(event Input|ActionEvents|InputActionFire!
  (params (Key :type Key%20Structure :default "None"))
  ;[0.05404 0.15 0.08285 0.5] Fire cannon with delay to time the animation
  (:Pressed
    (Utilities|FlowControl|DoOnce false
      (:Completed
        (Components|Animation|PlayAnimation (Variables|Default|GetCannonBody) "/Game/Characters+Objects/Objects/Cannon/CANNNON_Anim_Montage.CANNNON_Anim_Montage" false)
        (Utilities|FlowControl|Delay 1.2)
        (CallFunction|Refire)
        (CallFunction|FireCannon)))))

(event Input|ActionEvents|InputActionResetRotaion
  (params (Key :type Key%20Structure :default "None"))
  ;[1 0.0735 0] Resetting Cannon Rotation
  (:Pressed
    (Transformation|SetWorldRotation (Variables|Default|GetCannonBody) (Variables|Default|GetInitialRotation) false false)))

(event Input|ActionEvents|InputActionAimingAssist
  (params (Key :type Key%20Structure :default "None"))
  (bind _aimbeam (Variables|Default|GetAimBeam))
  ;[0.4167 0.009565 0] Aiming Assist Input
  (:Pressed
    (if (Variables|Default|GetAssistOn)
      (Variables|Default|SetAssistOn false)
      (Rendering|SetVisibility _aimbeam false false)
      (else
        (Variables|Default|SetAssistOn true)
        (Rendering|SetVisibility _aimbeam true false)))))

(event Input|AxisEvents|InputAxisTurn
  (params (AxisValue :type Float%20%28single-precision%29))
  ;[0.1971 0.2816 1] Cannon Aiming
  (Transformation|AddLocalRotation (Variables|Default|GetBasePivot) (Math|Rotator|MakeRotator 0.0 0.0 AxisValue) false false))

(event Input|AxisEvents|InputAxisLookUp
  (params (AxisValue :type Float%20%28single-precision%29))
  ;[0.1971 0.2816 1] Cannon Aiming
  (Transformation|AddLocalRotation (Variables|Default|GetBasePivot) (Math|Rotator|MakeRotator AxisValue 0.0 0.0) false false))

(fn ConstructionScript)