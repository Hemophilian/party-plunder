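; BP_TargetsShips is a shootable moving target in Oh_Ship, shown on a plane as a red, blue or green ship or a sea serpent.
; On BeginPlay it registers with BP_OhShipGameMode, picks a random look, delay and speed, then a timeline slides it along its right vector.
; TakingFire destroys the actor, then calls a delayed spawn of BP_Targets at the starting location, with the Delay placed after DestroyActor.
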(event Custom|Taking%20Fire!
  ;[1 0.02296 0] Target destroyed
  (Actor|DestroyActor)
  (Utilities|FlowControl|Delay 1.0)
  (Game|SpawnActorfromClass "/Game/Oh_Ship/Targets/BP_Targets.BP_Targets_C" (Math|Transform|MakeTransform (Variables|Default|GetBeginingLocation) "0, 0, 0" "2.500000,2.500000,2.500000") "Undefined" "MultiplyWithRoot" 0 0))

(event Custom|Setting%20Mesh
  ;[1 0 0.7459] Setting Colour/Mesh
  (if (Utilities|Enum|Equal(Enum) (Variables|Default|GetTarget%20Colour) "NewEnumerator0")
    (Rendering|Material|SetMaterial (Variables|Default|GetPlane) 0 "/Game/Oh_Ship/2D_stuff/RedShip_Mat.RedShip_Mat")
    (elif (Utilities|Enum|Equal(Enum) (Variables|Default|GetTarget%20Colour) "NewEnumerator1")
      (Rendering|Material|SetMaterial (Variables|Default|GetPlane) 0 "/Game/Oh_Ship/2D_stuff/BlueSHip_Mat.BlueSHip_Mat")
      (elif (Utilities|Enum|Equal(Enum) (Variables|Default|GetTarget%20Colour) "NewEnumerator2")
        (Rendering|Material|SetMaterial (Variables|Default|GetPlane) 0 "/Game/Oh_Ship/2D_stuff/GreenShip_Mat.GreenShip_Mat")
        (elif (Utilities|Enum|Equal(Enum) (Variables|Default|GetTarget%20Colour) "NewEnumerator3")
          (Rendering|Material|SetMaterial (Variables|Default|GetPlane) 0 "/Game/Oh_Ship/2D_stuff/SeaSerpent_Mat.SeaSerpent_Mat"))))))

(event Custom|SlowestMovement
  ;[0.1971 0.2816 1] Target Movement (10secs)
  (bind _output_get (Variables|Default|SetStartLocation (Transformation|GetActorLocation)))
  (Utilities|FlowControl|Delay (Variables|Default|GetMoveDelay))
  (bind _movetrack (Timeline|10SecTimeline Play)
    (:Update
      (Transformation|SetActorLocation (+ (* (* (Transformation|GetActorRightVector) (* _movetrack (Variables|Default|GetMoveSpeed))) (Variables|Default|GetMoveDistance)) _output_get) false false))))

(event EventBeginPlay
  ;[0.1971 0.2816 1] Picks random num (0-5) for movement delay
  (Variables|Default|SetMoveDelay (Math|Random|RandomFloatinRange 0.0 5.0))
  ;[0.1971 0.2816 1] Picks random num (0-3) for movement speed
  (Variables|Default|SetMoveSpeed (Math|Random|RandomFloatinRange 0.0 3.0))
  (bind _asbp_oh_ship_game_mode (Utilities|Casting|CastToBP_OhShipGameMode (Game|GetGameMode)))
  (Variables|/Game/Oh_Ship/BP_OhShipGameMode.BP_OhShipGameMode_C|SetAs%20BP%20TargetShips _asbp_oh_ship_game_mode self)
  (Variables|Default|SetBeginingLocation (Transformation|GetActorLocation))
  (Variables|Default|SetTarget%20Colour (.OutItem (Utilities|Array|Random (Utilities|Array|MakeArray "NewEnumerator0" "NewEnumerator2" "NewEnumerator1" "NewEnumerator3"))))
  (CallFunction|SettingMesh)
  (CallFunction|SlowestMovement))

(fn ConstructionScript)