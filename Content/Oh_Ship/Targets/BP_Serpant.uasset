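; BP_Serpant is a serpent actor that slides between a beginning and a target location supplied by the player's BP_Cannon pawn.
; BeginPlay caches both locations from the cannon and starts the movement state that heads for the target.
; Tick uses VInterpTo without sweep to ease toward the target, hold still, or return to the beginning, depending on that state.
; Nothing in this Blueprint changes the state after BeginPlay.
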(event EventTick
  (params (DeltaSeconds :type Float%20%28single-precision%29))
  ;[0.1971 0.2816 1] Moving the snake
  (if (Utilities|Enum|Equal(Enum) (Variables|Default|GetMovementState) "NewEnumerator0")
    (Transformation|SetActorLocation (Math|Interpolation|VInterpTo (Transformation|GetActorLocation) (Variables|Default|GetTargetLocation) (Utilities|Time|GetWorldDeltaSeconds) 5.0) false false)
    (elif (not (Utilities|Enum|Equal(Enum) (Variables|Default|GetMovementState) "NewEnumerator1"))
      (if (Utilities|Enum|Equal(Enum) (Variables|Default|GetMovementState) "NewEnumerator2")
        (Transformation|SetActorLocation (Math|Interpolation|VInterpTo (Transformation|GetActorLocation) (Variables|Default|GetBeginingLocation) (Utilities|Time|GetWorldDeltaSeconds) 5.0) false false)))))

(event EventBeginPlay
  ;[1 0.8856 0] Getting target location
  (bind _asbp_cannon (Utilities|Casting|CastToBP_Cannon (Game|Player|GetPlayerPawn 0)))
  (Variables|Default|SetTargetLocation (Variables|/Game/Oh_Ship/PlayerCharacters/BP_Cannon.BP_Cannon_C|GetTargetSerpantLocation _asbp_cannon))
  (Variables|Default|SetBeginingLocation (Variables|/Game/Oh_Ship/PlayerCharacters/BP_Cannon.BP_Cannon_C|GetBeginingSerpantLocation _asbp_cannon))
  (Variables|Default|SetMovementState "NewEnumerator0"))

(fn ConstructionScript)