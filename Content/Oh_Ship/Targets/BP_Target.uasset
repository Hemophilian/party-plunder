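; BP_Target is a moving shooting-target actor that is destroyed when it takes fire.
; On BeginPlay it stores its start location and plays the CarnivalRaleMovement timeline, offsetting itself along its right vector without sweep.
; MoveSpeed and MoveDistance both multiply the timeline's track value, so both scale the offset rather than the playback rate.
; The TakingFire! event destroys the actor after a short delay.
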(event Custom|Taking%20Fire!
  (Utilities|FlowControl|Delay 0.2)
  (Actor|DestroyActor))

(event EventBeginPlay
  (bind _output_get (Variables|Default|SetStartLocation (Transformation|GetActorLocation)))
  (bind _movetrack (Timeline|Carnival%20Rale%20Movement Play)
    (:Update
      (Transformation|SetActorLocation (+ (* (* (Transformation|GetActorRightVector) (* _movetrack (Variables|Default|GetMoveSpeed))) (Variables|Default|GetMoveDistance)) _output_get) false false))))

(event Collision|EventActorBeginOverlap
  (params (OtherActor :type Actor%20Object%20Reference)))

(event EventTick
  (params (DeltaSeconds :type Float%20%28single-precision%29)))

(fn ConstructionScript)