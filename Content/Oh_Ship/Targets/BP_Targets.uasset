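; BP_Targets is a shootable target in the Oh Ship game that respawns after it is hit.
; On BeginPlay it registers itself with BP_OhShipGameMode, saves its location and picks a random TargetColour, which selects a mesh, a material or a Plane shown in its place.
; TakingFire! turns on physics, then after a short delay destroys the actor and spawns a scaled replacement at the saved location, which rolls a new type.
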(event Custom|Taking%20Fire!
  ;[1 0.02296 0] Target destroyed
  (Physics|SetSimulatePhysics (Variables|Default|GetTarget) true)
  (Utilities|FlowControl|Delay 3.0)
  (Actor|DestroyActor)
  (Game|SpawnActorfromClass "BP_Targets_C" (Math|Transform|MakeTransform (Variables|Default|GetBeginingLocation) "0, 0, 0" "2.500000,2.500000,2.500000") "Undefined" "MultiplyWithRoot" 0 0))

(event Custom|Setting%20Target%20Type
  (bind _target (Variables|Default|GetTarget))
  ;[1 0 0.7459] Setting Target Type
  (if (Utilities|Enum|Equal(Enum) (Variables|Default|GetTarget%20Colour) "NewEnumerator0")
    (Components|StaticMesh|SetStaticMesh _target "/Game/Oh_Ship/3D_Stuff/Target.Target")
    (elif (Utilities|Enum|Equal(Enum) (Variables|Default|GetTarget%20Colour) "NewEnumerator1")
      (Components|StaticMesh|SetStaticMesh _target "/Game/Oh_Ship/3D_Stuff/target2.target2")
      (elif (Utilities|Enum|Equal(Enum) (Variables|Default|GetTarget%20Colour) "NewEnumerator2")
        (Rendering|Material|SetMaterial (Variables|Default|GetTarget) 0 "/Game/Characters+Objects/Objects/Material_001.Material_001")
        (elif (Utilities|Enum|Equal(Enum) (Variables|Default|GetTarget%20Colour) "NewEnumerator3")
          (Rendering|SetVisibility (Variables|Default|GetPlane) true false)
          (Rendering|SetVisibility (Variables|Default|GetTarget) false false))))))

(event EventBeginPlay
  ;[1 0.0735 0] Assinging variable values and Target Colour
  (bind _asbp_oh_ship_game_mode (Utilities|Casting|CastToBP_OhShipGameMode (Game|GetGameMode)))
  (Variables|/Game/Oh_Ship/BP_OhShipGameMode.BP_OhShipGameMode_C|SetAs%20BP%20Targets _asbp_oh_ship_game_mode self)
  (Variables|Default|SetBeginingLocation (Transformation|GetActorLocation))
  (Variables|Default|SetTarget%20Colour (.OutItem (Utilities|Array|Random (Utilities|Array|MakeArray "NewEnumerator0" "NewEnumerator2" "NewEnumerator1" "NewEnumerator3"))))
  (CallFunction|SettingTargetType))

(fn ConstructionScript)