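; Game mode for Oh Ship that runs a timed match, from opening countdown to winner screen.
; BeginPlay plays the countdown widget; StartGameTimer starts a looping tick that updates the timer display.
; At 60 or below, each tick re-arms the timer at a 0.2-second interval and adds another alert widget.
; At zero, EndMatch picks the cannon with the most Hits, shows its player and score, then pauses after a delay.
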(event Custom|StartGameTimer
  ;[0 0.15 0.149 0.5] The round timer
  (Variables|Default|SetIsMatchRunning true)
  (bind _returnvalue (UserInterface|CreateWidget "/Game/Oh_Ship/WBP_OhShipGameTimer.WBP_OhShipGameTimer_C"))
  (bind _output_get (Variables|Default|SetGame%20Timer _returnvalue))
  (UserInterface|Viewport|AddtoViewport _output_get 0)
  (Utilities|Time|SetTimerbyFunctionName 0 "TickMatchTimer" 1.0 true))

(event Custom|TickMatchTimer
  ;[0 0.15 0.149 0.5] The Timer
  (bind _output_get (Variables|Default|SetMatchTime (- (Variables|Default|GetMatchTime) 1)))
  (bind _output_get_2 (Variables|Default|SetMinutes (/ _output_get 60)))
  (bind _output_get_3 (Variables|Default|SetSeconds (Math|Integer|%(Integer) _output_get 60)))
  (if (Utilities|IsValid (Variables|Default|GetGame%20Timer))
    (Default|UpdateTimerDisplay (Variables|Default|GetGame%20Timer) _output_get_2 _output_get_3)
    (if (<= (Variables|Default|GetMatchTime) 0)
      (CallFunction|EndMatch)
      (elif (<= (Variables|Default|GetMatchTime) 60)
        (Utilities|Time|SetTimerbyFunctionName 0 "TickMatchTimer" 0.2 true)
        (bind _returnvalue (UserInterface|CreateWidget "/Game/Oh_Ship/WBP_OhShipTimerAlert.WBP_OhShipTimerAlert_C"))
        (UserInterface|Viewport|AddtoViewport _returnvalue 0)))))

(event Custom|EndMatch
  ;[0 0.15 0.149 0.5] The Round Finished
  (Utilities|Time|ClearTimerbyFunctionName 0 "TickMatchTimer")
  (Variables|Default|SetIsMatchRunning false)
  (bind _outactors (Actor|GetAllActorsOfClass "/Game/Oh_Ship/PlayerCharacters/BP_Cannon.BP_Cannon_C"))
  (for _array_element _outactors
    (if (> (Variables|/Game/Oh_Ship/PlayerCharacters/BP_Cannon.BP_Cannon_C|GetHits _array_element) (Variables|Default|GetWinningHits))
      (Variables|Default|SetWinningHits (Variables|/Game/Oh_Ship/PlayerCharacters/BP_Cannon.BP_Cannon_C|GetHits _array_element))
      (Variables|Default|SetWinningPlayer _array_element)
      (else
        (Development|PrintString "Dirt Cleaned isnt greater than Winning Dirt CLeaned"))))
  (bind _returnvalue (UserInterface|CreateWidget "/Game/Oh_Ship/WBP_OhShipFinished.WBP_OhShipFinished_C"))
  (Variables|/Game/Oh_Ship/WBP_OhShipFinished.WBP_OhShipFinished_C|SetWinnerPlayerName _returnvalue (Utilities|String|StringToName (Variables|/Game/Oh_Ship/PlayerCharacters/BP_Cannon.BP_Cannon_C|GetPlayer (Variables|Default|GetWinningPlayer))))
  (Variables|/Game/Oh_Ship/WBP_OhShipFinished.WBP_OhShipFinished_C|SetWinnerPlayerGold _returnvalue (Variables|Default|GetWinningHits))
  (UserInterface|Viewport|AddtoViewport _returnvalue 0)
  (Utilities|FlowControl|Delay 1.0)
  (Game|SetGamePaused true))

(event EventBeginPlay
  ;[0 0.15 0.149 0.5] Starts the Begining countdown
  (bind _returnvalue (UserInterface|CreateWidget "/Game/Oh_Ship/WBP_OhShipCountdown.WBP_OhShipCountdown_C"))
  (bind _output_get (Variables|Default|SetCountdownWidget _returnvalue))
  (UserInterface|Viewport|AddtoViewport _output_get 0)
  (Default|PlayCountdown _output_get))

(fn ConstructionScript)