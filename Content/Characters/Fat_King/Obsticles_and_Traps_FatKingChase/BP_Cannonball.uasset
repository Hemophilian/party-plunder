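; BP_Cannonball is a carryable cannonball, apparently for the Fat King chase, that registers itself with every BP_TopDownCharacter on BeginPlay.
; PickedUp disables physics and collision, attaches it to the character's CarryPoint and flags that character as carrying.
; Shockwave, gated by IsShockwaveActive, sphere-overlaps nearby characters, calling ForceDropAndStun on the stored last carrier per hit rather than each overlapped actor, then clears the flag after a delay.
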(event Custom|PickedUp
  (params (PickerUpper :type Object%20Object%20Reference))
  ;[0.15 0 0 0.5] Being Picked Up
  (bind _asbp_top_down_character (Utilities|Casting|CastToBP_TopDownCharacter PickerUpper))
  (Variables|Default|SetAs%20BP%20Top%20Down%20Character _asbp_top_down_character)
  (Physics|SetSimulatePhysics (Variables|Default|Getball) false)
  (Collision|SetCollisionEnabled (Variables|Default|GetSphere) "NoCollision")
  (Transformation|AttachComponentToComponent self (Variables|/Game/TopDown/Blueprints/FatKingChase_Blueprints/BP_TopDownCharacter.BP_TopDownCharacter_C|GetCarryPoint _asbp_top_down_character) "None" "SnapToTarget" "SnapToTarget" "KeepWorld" true)
  (Development|PrintString "Cannonball Picked Up" true true "(R=0.000000,G=0.000000,B=0.000000,A=1.000000)")
  (Variables|/Game/TopDown/Blueprints/FatKingChase_Blueprints/BP_TopDownCharacter.BP_TopDownCharacter_C|SetIsCarryingCannonBall _asbp_top_down_character true))

(event Custom|Shockwave
  ;[0 0.1549 0.4062] Shockwave locgic, when a cannonal hits the gorwnd it creates a shockwave
  (if (Variables|Default|GetIsShockwaveActive)
    (bind _outactors (Collision|SphereOverlapActors "0, 0, 0" 3e+02 (Utilities|Array|MakeArray "ObjectTypeQuery3") "/Game/TopDown/Blueprints/FatKingChase_Blueprints/BP_TopDownCharacter.BP_TopDownCharacter_C"))
    (for _array_element _outactors
      (Default|ForceDropandStun (Variables|Default|GetAs%20BP%20Top%20Down%20Character)))
    (Development|PrintString "Cannonball shockwave!!" true true "(R=0.406250,G=0.233866,B=0.000000,A=1.000000)")
    (Utilities|FlowControl|Delay 3.0)
    (Variables|Default|SetIsShockwaveActive false)))

(event EventBeginPlay
  ;[0.15 0.15 1 0.5] Assignng Referances
  (bind _outactors (Actor|GetAllActorsOfClass "/Game/TopDown/Blueprints/FatKingChase_Blueprints/BP_TopDownCharacter.BP_TopDownCharacter_C"))
  (for _array_element _outactors
    (bind _asbp_top_down_character (Utilities|Casting|CastToBP_TopDownCharacter _array_element))
    (Variables|/Game/TopDown/Blueprints/FatKingChase_Blueprints/BP_TopDownCharacter.BP_TopDownCharacter_C|SetCannonball _asbp_top_down_character self)))

(fn ConstructionScript)