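; Character select pedestal that displays and locks in a player's character choice in the main menu.
; Scroll events cycle a wrapping index through four skeletal meshes on the display until the choice is confirmed.
; Confirmation writes the index to the BP_GameInstance slot matching AssignedControllerID, shows the Ready indicator and blocks further scrolling.
; BeginPlay resets AssignedControllerID to 0, hides Ready and shows the initial character.
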(event Custom|ScrollLeft
  ;[1 0.1011 0.5926] Scrolling left and right through character options
  (if (not (Variables|Default|GetHasConfirmed))
    (bind _output_get (Variables|Default|SetCurrentCharacterIndes (- (Variables|Default|GetCurrentCharacterIndes) 1)))
    (if (< _output_get 0)
      (Variables|Default|SetCurrentCharacterIndes 3))
    (CallFunction|UpdateDisplayCharacter)
    (Development|PrintString (Utilities|String|ToString(Integer) (Variables|Default|GetCurrentCharacterIndes)) true true "(R=1.000000,G=0.047000,B=0.000000,A=1.000000)")))

(event Custom|ScrollRight
  ;[1 0.1011 0.5926] Scrolling left and right through character options
  (if (not (Variables|Default|GetHasConfirmed))
    (bind _output_get (Variables|Default|SetCurrentCharacterIndes (+ (Variables|Default|GetCurrentCharacterIndes) 1)))
    (if (> _output_get 3)
      (Variables|Default|SetCurrentCharacterIndes 0))
    (CallFunction|UpdateDisplayCharacter)
    (Development|PrintString (Utilities|String|ToString(Integer) (Variables|Default|GetCurrentCharacterIndes)) true true "(R=0.000000,G=1.000000,B=0.405329,A=1.000000)")))

(event Custom|UpdateDisplayCharacter
  (bind _charactermeshes (Variables|Default|GetCharacterMeshes))
  (bind _currentcharacterindes (Variables|Default|GetCurrentCharacterIndes))
  (bind _output (Utilities|Array|Get(acopy) _charactermeshes _currentcharacterindes))
  ;[1 0.1011 0.5926] Updating which character should be shown on the rotar
  (Components|SkeletalMesh|SetSkeletalMeshAsset (Variables|Default|GetCharacterDisplay) _output)
  (Development|PrintString (Utilities|GetDisplayName _output)))

(event Custom|CharacterConfirmation
  (bind _currentcharacterindes (Variables|Default|GetCurrentCharacterIndes))
  ;[1 0.1011 0.5926] Character confirmation and assignment to global value
  (bind _asbp_game_instance (Utilities|Casting|CastToBP_GameInstance (Game|GetGameInstance)))
  (switch int (Variables|Default|GetAssignedControllerID)
    (:0
      (bind _output_get (Variables|/Game/Main_Menu/Character_Select_BP/BP_GameInstance.BP_GameInstance_C|SetPlayer1_Character _asbp_game_instance _currentcharacterindes))
      (Development|PrintString (Utilities|String|ToString(Integer) _output_get)))
    (:1
      (bind _output_get_2 (Variables|/Game/Main_Menu/Character_Select_BP/BP_GameInstance.BP_GameInstance_C|SetPlayer2_Character _asbp_game_instance _currentcharacterindes))
      (Development|PrintString (Utilities|String|ToString(Integer) _output_get_2)))
    (:2
      (bind _output_get_3 (Variables|/Game/Main_Menu/Character_Select_BP/BP_GameInstance.BP_GameInstance_C|SetPlayer3_Character _asbp_game_instance _currentcharacterindes))
      (Development|PrintString (Utilities|String|ToString(Integer) _output_get_3)))
    (:3
      (bind _output_get_4 (Variables|/Game/Main_Menu/Character_Select_BP/BP_GameInstance.BP_GameInstance_C|SetPlayer4_Character _asbp_game_instance _currentcharacterindes))
      (Development|PrintString (Utilities|String|ToString(Integer) _output_get_4))))
  (Rendering|SetVisibility (Variables|Default|GetReady) true false)
  (Variables|Default|SetHasConfirmed true))

(event EventBeginPlay
  (Variables|Default|SetAssignedControllerID 0)
  (CallFunction|UpdateDisplayCharacter)
  (Rendering|SetVisibility (Variables|Default|GetReady) false false))

(event Collision|EventActorBeginOverlap
  (params (OtherActor :type Actor%20Object%20Reference)))

(event EventTick
  (params (DeltaSeconds :type Float%20%28single-precision%29)))

(fn ConstructionScript)